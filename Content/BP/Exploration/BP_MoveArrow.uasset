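; BP_MoveArrow is an exploration navigation arrow that moves the player's view to another camera when clicked.
; On click, it checks TargetCamera and passes it to the player controller's SetViewTargetWithBlend.
; If no camera is assigned, it prints an on-screen warning instead.
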(event `/Game/BP/Props/BPI_InteractableObject.OnClickOn`
  (bind _targetcamera (`self.TargetCamera`))
  (if (!= _targetcamera null)
    (`PlayerController.SetViewTargetWithBlend` (`GameplayStatics.GetPlayerController` 0) _targetcamera 0.0 "VTBlend_Linear" 0.0 false)
    (else
      (`KismetSystemLibrary.PrintString` "Warning: no camera set on arrow" true true (struct :`R` 1.0 :`G` 0.908744 :`A` 1.0)))))

(fn `UserConstructionScript`
  (`parent.UserConstructionScript`))