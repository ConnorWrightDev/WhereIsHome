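; Clickable navigation arrow that blends the player's view to its assigned TargetCamera.
; It starts hidden, with Enable and Disable toggling visibility and query collision on the arrow body and head.
; A click has CON_Home blend cameras, bracketed by start and end calls that block interactions, printing warnings if camera or controller is invalid.
; The end call relies on a Delay matching BlendDuration, which can desync if the game pauses.
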(event `self.ReceiveBeginPlay`
  (`parent.ReceiveBeginPlay`)
  (`self.Disable`))

(event `/Game/BP/Props/BPI_InteractableObject.OnClickOn`
  (bind _blendduration (`self.BlendDuration`))
  (`parent.OnClickOn`)
  (if (!= (`self.TargetCamera`) null)
    (bind _ascon_home (cast `/Game/BP/Game/CON_Home` (`GameplayStatics.GetPlayerController` 0))
      (:`then`
        ;[1 1 1] Blend camera, disabling interactions during the whole transition. Pausing game make break the sync between blending inside Change Camera Blend and Delay, so be careful
        (`/Game/BP/Game/CON_Home.OnCameraBlendStart` _ascon_home)
        (`/Game/BP/Game/CON_Home.ChangeCamera_Blend` _ascon_home (`self.TargetCamera`) _blendduration)
        (`KismetSystemLibrary.Delay` _blendduration)
        (`/Game/BP/Game/CON_Home.OnCameraBlendEnd` _ascon_home))
      (:`CastFailed`
        (`KismetSystemLibrary.PrintString` "Warning: Player Controller is not a CON_Home" true true (struct :`R` 1.0 :`G` 0.908744 :`A` 1.0))))
    (else
      (`KismetSystemLibrary.PrintString` "Warning: no camera set on arrow" true true (struct :`R` 1.0 :`G` 0.908744 :`A` 1.0)))))

(fn `Disable`
  (bind _arrowbody (`self.ArrowBody`))
  (`PrimitiveComponent.SetCollisionEnabled` _arrowbody "NoCollision")
  (`PrimitiveComponent.SetCollisionEnabled` (`self.ArrowHead`) "NoCollision")
  (`SceneComponent.SetVisibility` _arrowbody false true)
  (`SceneComponent.SetVisibility` (`self.ArrowHead`) false true))

(fn `Enable`
  (bind _arrowbody (`self.ArrowBody`))
  (`PrimitiveComponent.SetCollisionEnabled` _arrowbody "QueryOnly")
  (`PrimitiveComponent.SetCollisionEnabled` (`self.ArrowHead`) "QueryOnly")
  (`SceneComponent.SetVisibility` _arrowbody true true)
  (`SceneComponent.SetVisibility` (`self.ArrowHead`) true true))

(fn `UserConstructionScript`
  (`parent.UserConstructionScript`))