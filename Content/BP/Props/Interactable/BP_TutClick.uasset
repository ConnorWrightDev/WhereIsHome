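; BP_TutClick is an interactable prop that responds to a click during what its message calls a tutorial.
; Its OnClickon event casts the player controller to CON_Home and updates the GUIBottomText widget with a wry line saying this is not an ending, just a tutorial.
; It has no other active logic, as the default events are disabled and construction only calls the parent.
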(event `/Game/BP/Props/BPI_InteractableObject.OnClickOn`
  (bind _ascon_home (cast `/Game/BP/Game/CON_Home` (`GameplayStatics.GetPlayerController` 0)))
  (`/Game/BP/UMG/UMG_BottomScreen.TextUpdate` (`/Game/BP/Game/CON_Home.GUI_BottomText` _ascon_home) "Very clever...but this isn't an ending. Just a tutorial."))

(fn `UserConstructionScript`
  (`parent.UserConstructionScript`))