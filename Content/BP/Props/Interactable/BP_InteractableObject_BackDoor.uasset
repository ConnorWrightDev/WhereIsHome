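; Interactable back door prop that triggers an ending and returns the player to the main menu.
; On click it runs the parent click logic, plays the FadeToBlack level sequence and shows the UMG_EndGame widget with a "home" ending line.
; After a short delay it loads MenuLevel.
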(event `/Game/BP/Props/BPI_InteractableObject.OnClickOn`
  (`parent.OnClickOn`)
  (bind (_outactor _returnvalue) (`LevelSequencePlayer.CreateLevelSequencePlayer` "/Game/FadeToBlack.FadeToBlack"))
  (`MovieSceneSequencePlayer.Play` _returnvalue)
  (bind _returnvalue_2 (`|CreateWidget` "/Game/BP/UMG/UMG_EndGame.UMG_EndGame_C" (`GameplayStatics.GetPlayerController` 0)))
  (`TextBlock.SetText` (`/Game/BP/UMG/UMG_EndGame.HomeKeyEndingText` _returnvalue_2) "Home is.... where you came from.")
  (`UserWidget.AddToViewport` _returnvalue_2 0)
  (`KismetSystemLibrary.Delay` 5.0)
  (`GameplayStatics.OpenLevel` "MenuLevel"))

(fn `UserConstructionScript`
  (`parent.UserConstructionScript`))