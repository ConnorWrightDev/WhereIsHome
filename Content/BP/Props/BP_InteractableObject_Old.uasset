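; Interactable prop Blueprint that changes its highlight color in response to hover and click events.
; The construction script gives each static mesh component a dynamic material instance on slot 0, setting its base color and an index-matched texture, with a fallback texture.
; Events pass a state name to AppearanceStateUpdate, which looks it up in the Colors map, falling back to Default, and applies it to every stored instance.
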(event `/Game/BP/Props/BPI_InteractableObject.OnHoverOn`
  (`self.AppearanceStateUpdate` "OnHover"))

(event `/Game/BP/Props/BPI_InteractableObject.OnHoverOff`
  (`self.AppearanceStateUpdate` "Default"))

(event `/Game/BP/Props/BPI_InteractableObject.OnClickOn`
  (`self.AppearanceStateUpdate` "OnClick"))

(event `/Game/BP/Props/BPI_InteractableObject.OnClickOff`
  (`self.AppearanceStateUpdate` "Default"))

(fn `AppearanceStateUpdate`
  (params (State :type Name))
  (bind _colors (`self.Colors`))
  (bind (_value _returnvalue) (`BlueprintMapLibrary.Map_Find` _colors State))
  (for _array_element (`self.MI_Instances`)
    (`MaterialInstanceDynamic.SetVectorParameterValue` _array_element "HighlightColor" (`KismetMathLibrary.SelectColor` _value (`BlueprintMapLibrary.Map_Find` _colors "Default") _returnvalue)))
  (return))

(fn `UserConstructionScript`
  (bind _tex_textures (`self.TEX_Textures`))
  (for (_array_element _array_index) (`self.K2_GetComponentsByClass` "/Script/Engine.StaticMeshComponent")
    (bind _returnvalue (`PrimitiveComponent.CreateDynamicMaterialInstance` _array_element 0 "/Game/Art/Materials/MAT_InteractableObject.MAT_InteractableObject" "None"))
    (bind _output (`|GetArrayItem` _tex_textures _array_index))
    (`MaterialInstanceDynamic.SetTextureParameterValue` _returnvalue "Texture" (select `bool` (and (`KismetSystemLibrary.IsValid` _output) (< 0 (`KismetArrayLibrary.Array_Length` _tex_textures))) :`false` "/Game/Art/Textures/noTexture.noTexture" :`true` _output :!type "Texture Object Reference"))
    (`KismetArrayLibrary.Array_Add` (`self.MI_Instances`) _returnvalue)
    (`MaterialInstanceDynamic.SetVectorParameterValue` _returnvalue "BaseColor" (`self.BaseColor`)) ; Set base color
  ))